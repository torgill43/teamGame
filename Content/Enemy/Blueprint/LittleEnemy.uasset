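; LittleEnemy is an enemy cube that shuttles along a timeline-driven path until it is hit.
; The Moving timeline sets the cube's relative location, while a delay in its update flips IsLooped to alternate forward and reverse playback.
; Any hit hides the cube, disables its collision, spawns the fracturable Enemy_static at its transform and destroys the actor.
; Leftover respawn and transform nodes are unconnected.
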(event `self.ReceiveBeginPlay`
  (bind (_direction __) (`Timeline|Moving` :!label _label)
    (:`Update`
      (`SceneComponent.K2_SetRelativeLocation` (`self.Cube`) __ false false)
      (`KismetSystemLibrary.Delay` 3.0)
      (if (`self.IsLooped`)
        (set `self.IsLooped` false) ; Loops in reverse once enemy made it to end point
        (goto _label :!via `Reverse`)
        (else
          (set `self.IsLooped` true) ; Loops from beginning again
          (goto _label))))))

(event `self.ReceiveTick`
  (params (DeltaSeconds :type "Float (single-precision)")))

(event `self.ReceiveHit`
  (params (MyComp :type "PrimitiveComponent Object Reference") (Other :type "Actor Object Reference") (OtherComp :type "PrimitiveComponent Object Reference") (bSelfMoved :type Boolean) (HitLocation :type "Vector Structure") (HitNormal :type "Vector Structure") (NormalImpulse :type "Vector Structure") (Hit :type "HitResult Structure (by ref)"))
  (bind _cube (`self.Cube`))
  (bind (_returnvalue_location _returnvalue_rotation _returnvalue_scale) (`KismetMathLibrary.BreakTransform` (`SceneComponent.K2_GetComponentToWorld` _cube)))
  ;[1 1 1] Spans the destructable actor when the "0 " key is pressed (in theory)
  (`SceneComponent.SetHiddenInGame` _cube true false)
  (`PrimitiveComponent.SetCollisionEnabled` _cube "NoCollision")
  (`|SpawnActorFromClass` "/Game/sierra_testing/Enemy_static.Enemy_static_C" (`KismetMathLibrary.MakeTransform` _returnvalue_location _returnvalue_rotation _returnvalue_scale) "Undefined" "OverrideRootScale" null null) ; spawns the static mesh which can be fractured
  (`self.K2_DestroyActor`) ; place at end
)

(fn `UserConstructionScript`)