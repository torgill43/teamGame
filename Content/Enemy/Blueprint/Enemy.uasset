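; Enemy character that chases the player on sight, plays a melee counter-punch, and breaks apart when hit.
; PawnSensing triggers an AI move to the player, then a punch montage gated by CanAttack for the montage's length.
; A separate left-mouse Attack adds a debug line trace whose result is unused.
; Any Hit event hides the mesh, spawns fracturable Enemy_static at its transform, and destroys the actor.
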(event `self.ReceiveTick`
  (params (DeltaSeconds :type "Float (single-precision)")))

(event `Key|LeftMouseButton`
  (params (Key :type "Key Structure"))
  (:`Pressed`
    (`self.Attack`)))

(event `self.PawnSensing.OnSeePawn`
  (params (Pawn :type "Pawn Object Reference"))
  (set `self.IsSeeingPlayer?` true)
  (`self.FollowPlayer`))

(event `Attack`
  (`self.PlayAnimMontage` "/Game/Enemy/Animations/Paired_CounterPunch_PalmStrike_Att_Montage.Paired_CounterPunch_PalmStrike_Att_Montage")
  (`KismetSystemLibrary.LineTraceSingle` :`Start` (`SceneComponent.GetSocketLocation` (`self.StartAttack`) "None") :`End` (`SceneComponent.GetSocketLocation` (`self.EndAttack`) "None") :`TraceChannel` "TraceTypeQuery1" :`DrawDebugType` "ForDuration"))

(event `FollowPlayer`
  (if (`self.IsSeeingPlayer?`)
    (`|AIMoveTo` self (0.0 0.0 0.0) (`GameplayStatics.GetPlayerCharacter` 0) 70.0
      (:`then`
        (if (`self.canAttack?`)
          (set `self.canAttack?` false)
          (bind _returnvalue (`self.PlayAnimMontage` "/Game/Enemy/Animations/Paired_CounterPunch_PalmStrike_Att_Montage.Paired_CounterPunch_PalmStrike_Att_Montage"))
          (`KismetSystemLibrary.Delay` _returnvalue)
          (set `self.canAttack?` true))))))

(event `self.ReceiveHit`
  (params (MyComp :type "PrimitiveComponent Object Reference") (Other :type "Actor Object Reference") (OtherComp :type "PrimitiveComponent Object Reference") (bSelfMoved :type Boolean) (HitLocation :type "Vector Structure") (HitNormal :type "Vector Structure") (NormalImpulse :type "Vector Structure") (Hit :type "HitResult Structure (by ref)"))
  (bind _mesh (`self.Mesh`))
  (bind (_returnvalue_location _returnvalue_rotation _returnvalue_scale) (`KismetMathLibrary.BreakTransform` (`SceneComponent.K2_GetComponentToWorld` _mesh)))
  ;[1 1 1] Spans the destructable actor when the "0 " key is pressed (in theory)
  (`SceneComponent.SetHiddenInGame` _mesh true false)
  (`PrimitiveComponent.SetCollisionEnabled` _mesh "NoCollision")
  (`|SpawnActorFromClass` "/Game/sierra_testing/Enemy_static.Enemy_static_C" (`KismetMathLibrary.MakeTransform` _returnvalue_location _returnvalue_rotation _returnvalue_scale) "Undefined" "OverrideRootScale" null null) ; spawns the static mesh which can be fractured
  (`self.K2_DestroyActor`) ; place at end
)

(fn `UserConstructionScript`)